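; BP_AVI_Master is a configurable static mesh actor from the ArchVisIndustrial content, exposing wood and metal material adjustments.
; The construction script creates a dynamic instance of M_AVI on the mesh's first material slot.
; It feeds the actor's variables into that instance to set tint, roughness, metal adjustment, and detail texture scale, intensity and rotation.
; The event graph holds only disabled stub events, so nothing runs at gameplay time.
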(event `self.ReceiveBeginPlay`)

(event `self.ReceiveActorBeginOverlap`
  (params (OtherActor :type "Actor Object Reference")))

(event `self.ReceiveTick`
  (params (DeltaSeconds :type "Float (single-precision)")))

(fn `UserConstructionScript`
  (bind _returnvalue (`PrimitiveComponent.CreateDynamicMaterialInstance` (`self.StaticMesh`) 0 "/Game/ArchVisIndustrial/Materials/M_AVI.M_AVI"))
  (`MaterialInstanceDynamic.SetVectorParameterValue` _returnvalue "WoodTint" (`self.WoodTint`))
  (`MaterialInstanceDynamic.SetVectorParameterValue` _returnvalue "MetalTint" (`self.MetalTint`))
  (`MaterialInstanceDynamic.SetScalarParameterValue` _returnvalue "MetalAdjustment" (`self.MetalAdjustment`))
  (`MaterialInstanceDynamic.SetScalarParameterValue` _returnvalue "WoodRoughnessAdjustment" (`self.WoodRoughnessAdjustment`))
  (`MaterialInstanceDynamic.SetScalarParameterValue` _returnvalue "MetalRoughnessAdjustment" (`self.MetalRoughnessAdjustment`))
  (`MaterialInstanceDynamic.SetTextureParameterValue` _returnvalue "WoodDetailTexture" (`self.WoodDetailTexture`))
  (`MaterialInstanceDynamic.SetScalarParameterValue` _returnvalue "WoodDetailUVScale" (`self.WoodDetailUVScale`))
  (`MaterialInstanceDynamic.SetVectorParameterValue` _returnvalue "WoodDetailIntensity" (`self.WoodDetailIntensity`))
  (`MaterialInstanceDynamic.SetScalarParameterValue` _returnvalue "WoodDetailRotation" (`self.WoodDetailRotation`))
  (`MaterialInstanceDynamic.SetTextureParameterValue` _returnvalue "MetalDetailTexture" (`self.MetalDetailTexture`))
  (`MaterialInstanceDynamic.SetScalarParameterValue` _returnvalue "MetalDetailUVScale" (`self.MetalDetailUVScale`))
  (`MaterialInstanceDynamic.SetVectorParameterValue` _returnvalue "MetalDetailIntensity" (`self.MetalDetailIntensity`))
  (`MaterialInstanceDynamic.SetScalarParameterValue` _returnvalue "MetalDetailRotation" (`self.MetalDetailRotation`)))