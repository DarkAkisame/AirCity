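; Sword pickup actor that lets the first-person player take the weapon by pressing E while in range.
; Capsule overlap enables input from player controller 0 and sets CanPickUP for any overlapping actor, and end overlap reverses both.
; On E, it casts the actor from the begin-overlap event to FirstPersonCharacter and passes its static mesh component to PickUpWeapon.
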(event `self.Capsule.OnComponentBeginOverlap`
  (params (OverlappedComponent :type "PrimitiveComponent Object Reference") (OtherActor :type "Actor Object Reference") (OtherComp :type "PrimitiveComponent Object Reference") (OtherBodyIndex :type Integer) (bFromSweep :type Boolean) (SweepResult :type "HitResult Structure (by ref)"))
  (`self.EnableInput` (`GameplayStatics.GetPlayerController` 0))
  (set `self.canPickUP` true))

(event `self.Capsule.OnComponentEndOverlap`
  (params (OverlappedComponent :type "PrimitiveComponent Object Reference") (OtherActor :type "Actor Object Reference") (OtherComp :type "PrimitiveComponent Object Reference") (OtherBodyIndex :type Integer))
  (`self.DisableInput` (`GameplayStatics.GetPlayerController` 0))
  (set `self.canPickUP` false))

(event `Key|E` :consume false
  (params (Key :type "Key Structure"))
  (:`Pressed`
    (if (`self.canPickUP`)
      (bind _asfirst_person_character (cast `/Game/FirstPersonBP/Blueprints/FirstPersonCharacter` (stale `self.Capsule.OnComponentBeginOverlap` OtherActor)))
      (`/Game/FirstPersonBP/Blueprints/FirstPersonCharacter.PickUpWeapon` _asfirst_person_character (`self.StaticMeshComponent`)))))

(fn `UserConstructionScript`)